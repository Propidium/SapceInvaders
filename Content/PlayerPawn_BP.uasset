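; Player pawn Blueprint that spawns the player's ship and keeps a count of ships.
; On BeginPlay it calls SpawnShips, marked TBD, which spawns one PlayerShip_BP at the world location of the ShipOrigin component.
; ReportPlayerShipDeath decrements NumShips and prints the remaining count.
; A node to attach to ShipOrigin is unconnected and never runs.
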(event `self.ReceiveBeginPlay`
  (`self.SpawnShips`))

(event `SpawnShips`
  ;[1 0.5832 0] TBD
  (`|SpawnActorFromClass` "/Game/PlayerShip_BP.PlayerShip_BP_C" (`KismetMathLibrary.MakeTransform` (`SceneComponent.K2_GetComponentLocation` (`self.ShipOrigin`))) "Undefined" "MultiplyWithRoot" null null))

(event `/Game/Interfaces/Sapce_Interface.Report Player Ship Death`
  (bind _output_get (set `self.NumShips` (- (`self.NumShips`) 1)))
  (`KismetSystemLibrary.PrintString` (`KismetStringLibrary.Conv_IntToString` _output_get)))

(fn `UserConstructionScript`)