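; Player ship actor that drops a bomb when clicked and can be damaged and destroyed.
; A reload timeline drives the Charge parameter on the plane's dynamic sprite material and re-arms the weapon when full, restarting after each shot.
; Explode spawns an effect and removes one health; at zero, Die notifies the player's pawn, detaches and destroys the ship.
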(event `self.ReceiveBeginPlay`
  (bind _returnvalue (`KismetMaterialLibrary.CreateDynamicMaterialInstance` "/Game/Assets/DrawSprite_M.DrawSprite_M"))
  (bind _output_get (set `self.DynamicMaterialRef` _returnvalue))
  (`PrimitiveComponent.SetMaterial` (`self.Plane`) 0 _output_get)
  (`self.Charge`))

(event `self.ReceiveActorOnClicked`
  (params (ButtonPressed :type "Key Structure"))
  (bind _returnvalue_location (`KismetMathLibrary.BreakTransform` (`self.GetTransform`)))
  ;[1 1 1] Fire Ship Weapon
  (if (`self.IsArmed`)
    (set `self.IsArmed` false)
    (`|SpawnActorFromClass` "/Game/Bomb_BP.Bomb_BP_C" (`KismetMathLibrary.MakeTransform` _returnvalue_location) "Undefined" "MultiplyWithRoot" null null)
    (`self.Charge`)))

(event `Charge`
  ;[1 1 1] Charge ship weapon, update charge meters
  (bind (_direction _newtrack_0) (`Timeline|ReloadTimer` :!via `PlayFromStart`)
    (:`Update`
      (`MaterialInstanceDynamic.SetScalarParameterValue` (`self.DynamicMaterialRef`) "Charge" _newtrack_0)
      (set `self.IsArmed` (>= _newtrack_0 1.0)))))

(event `/Game/Interfaces/Sapce_Interface.Explode`
  (params (NewParam :type Boolean))
  ;[1 1 1] TBD
  ;;[1 1 1] Play explosion animation
  (`|SpawnActorFromClass` "/Game/GreenExplosion.GreenExplosion_C" (`KismetMathLibrary.MakeTransform` (`self.K2_GetActorLocation` self)) "Undefined" "MultiplyWithRoot" null null)
  (bind _output_get (set `self.Health` (- (`self.Health`) 1)))
  (if (<= _output_get 0)
    (`self.Die`)))

(event `Die`
  ;[1 1 1] Die
  (message `/Game/Interfaces/Sapce_Interface.Report Player Ship Death` (`Controller.K2_GetPawn` (`GameplayStatics.GetPlayerController` 0)))
  (`self.K2_DetachFromActor` "KeepRelative")
  (`self.K2_DestroyActor`))

(fn `UserConstructionScript`)