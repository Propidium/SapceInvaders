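; Bomb actor that moves along negative world Y at an ever-increasing speed.
; Each Tick adds Acceleration to Speed and offsets the actor by that amount with a swept SetActorLocation, without scaling by delta time, so motion depends on frame rate.
; The overlap event is empty, and a class comparison against EnemyPawn_BP is left unconnected, so the bomb has no hit response.
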(event `self.ReceiveTick`
  (params (DeltaSeconds :type "Float (single-precision)"))
  (bind _output_get (set `self.Speed` (+ (`self.Acceleration`) (`self.Speed`))))
  (`self.K2_SetActorLocation` (`KismetMathLibrary.MakeVector` (.x (`self.K2_GetActorLocation`)) (- (.y (`self.K2_GetActorLocation`)) _output_get) (.z (`self.K2_GetActorLocation`))) true))

(event `self.ReceiveActorBeginOverlap`
  (params (OtherActor :type "Actor Object Reference")))

(fn `UserConstructionScript`)